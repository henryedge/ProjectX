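; A coffee cup prop that simulates physics and can be picked up and released.
; Pickup turns off physics and collision and snaps the cup mesh to the supplied holder component, while ReleaseObject detaches it and restores both.
; Both events then report the held state to player character 0 through a WasPickedUp interface message, flagged as a non-key item.
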(event `self.releaseObject`
  (`self.SetActorEnableCollision` true)
  (`self.DetachRootComponentFromParent` true)
  (`PrimitiveComponent.SetSimulatePhysics` (`self.coffee_cup`) true)
  (set `self.PickedUp` false)
  (message `/Game/Blueprints/BPI_sendlinetrace.wasPickedUp` (`GameplayStatics.GetPlayerCharacter` 0) (`self.PickedUp`) false 0 :!label _label))

(event `self.Pickup`
  (params (PickupHolder :type "SceneComponent Object Reference"))
  ;[1 1 1] Pickup item
  (`PrimitiveComponent.SetSimulatePhysics` (`self.coffee_cup`) false)
  (`self.SetActorEnableCollision` false)
  (`SceneComponent.K2_AttachTo` (`self.coffee_cup`) PickupHolder "None" "SnapToTarget" true)
  (set `self.PickedUp` true)
  (goto _label))

(fn `UserConstructionScript`
  (`PrimitiveComponent.SetSimulatePhysics` true))