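; Key-locked exterior door actor that swings open and closed when its OpenDoor event is called.
; OpenDoor looks up the door's Index in the passed Keys array, printing a message if the key is missing, otherwise toggling IsClosed.
; A DoorRotation timeline plays or reverses to lerp the door's relative yaw.
; The construction script derives both angles from the placed yaw, a quarter turn apart in the OpenClockwise direction.
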(event `self.ReceiveBeginPlay`)

(event `self.ReceiveActorBeginOverlap`
  (params (OtherActor :type "Actor Object Reference")))

(event `self.openDoor`
  (params (Keys :type "Array of Boolean (by ref)"))
  (if (`KismetArrayLibrary.Array_Get` Keys (`self.index`))
    (if (`self.isClosed`)
      (set `self.isClosed` false)
      (bind (_direction _doorrot) (`Timeline|DoorRotation` :!label _label)
        (:`Update`
          (`SceneComponent.K2_SetRelativeRotation` (`self.door`) (`KismetMathLibrary.MakeRot` 0.0 (`KismetMathLibrary.Lerp` (`self.closedRot`) (`self.openRot`) _doorrot)) false)))
      (else
        (set `self.isClosed` true)
        (goto _label :!via `Reverse`)))
    (else
      (`KismetSystemLibrary.PrintString` "You don't have the key for this door"))))

(fn `UserConstructionScript`
  (bind _yaw (.yaw (`SceneComponent.RelativeRotation` (`self.door`))))
  (set `self.closedRot` _yaw)
  (if (`self.openClockwise`)
    (set `self.openRot` (+ _yaw 90.0))
    (else
      (set `self.openRot` (- _yaw 90.0)))))