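; BP_sisäovi is an interior door that the player toggles open and closed with the left mouse button while inside its trigger box.
; Trigger overlaps enable and disable player input on the actor, without filtering the overlapping actor.
; The construction script derives open yaw as 90 degrees either way from the Door component's yaw, per OpenClockwise.
; A DoorRotation timeline plays or reverses, lerping the whole actor's relative yaw.
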(event `self.ReceiveBeginPlay`)

(event `self.ReceiveActorBeginOverlap`
  (params (OtherActor :type "Actor Object Reference")))

(event `self.ReceiveTick`
  (params (DeltaSeconds :type "Float (single-precision)")))

(event `self.TriggerBox.OnComponentBeginOverlap`
  (params (OtherActor :type "Actor Object Reference") (OtherComp :type "PrimitiveComponent Object Reference") (OtherBodyIndex :type Integer) (bFromSweep :type Boolean) (SweepResult :type "EngineTypes.HitResult Structure (by ref)"))
  (`self.EnableInput` (`GameplayStatics.GetPlayerController` 0)))

(event `self.TriggerBox.OnComponentEndOverlap`
  (params (OtherActor :type "Actor Object Reference") (OtherComp :type "PrimitiveComponent Object Reference") (OtherBodyIndex :type Integer))
  (`self.DisableInput` (`GameplayStatics.GetPlayerController` 0)))

(event `Key|LeftMouseButton`
  (:`Pressed`
    (if (`self.isClosed`)
      (set `self.isClosed` false)
      (bind (_direction _doorrot) (`Timeline|DoorRotation` :!label _label)
        (:`Update`
          (`self.K2_SetActorRelativeRotation` (`KismetMathLibrary.MakeRot` 0.0 (`KismetMathLibrary.Lerp` (`self.closedRot`) (`self.openRot`) _doorrot)))))
      (else
        (set `self.isClosed` true)
        (goto _label :!via `Reverse`)))))

(fn `UserConstructionScript`
  (bind _yaw (.yaw (`SceneComponent.RelativeRotation` (`self.door`))))
  (set `self.closedRot` _yaw)
  (if (`self.openClockwise`)
    (set `self.openRot` (+ _yaw 90.0))
    (else
      (set `self.openRot` (- _yaw 90.0)))))