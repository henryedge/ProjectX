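; Pickup_Cube is a physics-simulated object that can be picked up, carried and released.
; Pickup turns off physics and collision, then snaps the root component to the supplied holder.
; ReleaseObject restores collision, detaches the static mesh and re-enables physics.
; Both events update PickedUp and pass it to player character 0 through WasPickedUpMessage; the construction script enables physics and input.
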(event `self.releaseObject`
  (`self.SetActorEnableCollision` true)
  (`SceneComponent.DetachFromParent` (`self.StaticMeshComponent`) true)
  (`PrimitiveComponent.SetSimulatePhysics` true)
  (set `self.PickedUp` false)
  (message `/Game/Blueprints/BPI_sendlinetrace.wasPickedUp` (`GameplayStatics.GetPlayerCharacter` 0) (`self.PickedUp`) :!label _label))

(event `self.Pickup`
  (params (PickupHolder :type "SceneComponent Object Reference"))
  ;[1 1 1] Pickup item and attach it to right hand
  (`PrimitiveComponent.SetSimulatePhysics` false)
  (`self.SetActorEnableCollision` false)
  (`self.K2_AttachRootComponentTo` PickupHolder "None" "SnapToTarget")
  (set `self.PickedUp` true)
  (goto _label))

(event `self.ReceiveBeginPlay`)

(event `self.ReceiveActorBeginOverlap`
  (params (OtherActor :type "Actor Object Reference")))

(event `self.ReceiveTick`
  (params (DeltaSeconds :type "Float (single-precision)")))

(fn `UserConstructionScript`
  (`PrimitiveComponent.SetSimulatePhysics` true)
  (`self.EnableInput` null))